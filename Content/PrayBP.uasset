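; PrayBP is a prey actor that detects hunters through two trigger volumes, an outer and an inner detection zone.
; Begin and end overlap events on each volume cast the other actor to HunterBP and ignore anything else.
; Each event only prints a debug message, with no movement, flee or death logic implemented.
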(event OnComponentEndOverlap(HuntterDetectionOuter)
  (params (OverlappedComponent :type Primitive%20Component%20Object%20Reference) (OtherActor :type Actor%20Object%20Reference) (OtherComp :type Primitive%20Component%20Object%20Reference) (OtherBodyIndex :type Integer))
  (Utilities|Casting|CastToHunterBP OtherActor)
  (Development|PrintText "left detecton"))

(event OnComponentBeginOverlap(HuntterDetectionOuter)
  (params (OverlappedComponent :type Primitive%20Component%20Object%20Reference) (OtherActor :type Actor%20Object%20Reference) (OtherComp :type Primitive%20Component%20Object%20Reference) (OtherBodyIndex :type Integer) (bFromSweep :type Boolean) (SweepResult :type Hit%20Result%20Structure%20%28by%20ref%29))
  (Utilities|Casting|CastToHunterBP OtherActor)
  (Development|PrintText "entered detecton"))

(event OnComponentBeginOverlap(HuntterDetectionInner)
  (params (OverlappedComponent :type Primitive%20Component%20Object%20Reference) (OtherActor :type Actor%20Object%20Reference) (OtherComp :type Primitive%20Component%20Object%20Reference) (OtherBodyIndex :type Integer) (bFromSweep :type Boolean) (SweepResult :type Hit%20Result%20Structure%20%28by%20ref%29))
  (Utilities|Casting|CastToHunterBP OtherActor)
  (Development|PrintText "Go Me"))

(event OnComponentEndOverlap(HuntterDetectionInner)
  (params (OverlappedComponent :type Primitive%20Component%20Object%20Reference) (OtherActor :type Actor%20Object%20Reference) (OtherComp :type Primitive%20Component%20Object%20Reference) (OtherBodyIndex :type Integer))
  (Utilities|Casting|CastToHunterBP OtherActor)
  (Development|PrintText "I should be dead"))

(event EventBeginPlay)

(event Collision|EventActorBeginOverlap
  (params (OtherActor :type Actor%20Object%20Reference)))

(event EventTick
  (params (DeltaSeconds :type Float%20%28single-precision%29)))

(fn ConstructionScript)